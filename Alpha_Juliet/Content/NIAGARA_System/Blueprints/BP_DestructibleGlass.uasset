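; BP_DestructibleGlass is a glass wall actor that shatters when it takes any damage.
; On damage, it spawns the NS_DestructibleGlass Niagara effect at the intact mesh's transform, removes that mesh and plays a glass break sound.
; The actor destroys itself once the Niagara system reports that it has finished.
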(event Custom|Destroy_Glass
  (params (PSystem :type Niagara%20Component%20Object%20Reference))
  ;[1 1 1] Dammage with linetrace and destruction
  (Actor|DestroyActor))

(event Game|Damage|EventAnyDamage
  (params (Damage :type Float%20%28single-precision%29) (DamageType :type Damage%20Type%20Object%20Reference) (InstigatedBy :type Controller%20Object%20Reference) (DamageCauser :type Actor%20Object%20Reference))
  (bind _glasswall_nondestroyed (Variables|Default|GetGlassWall_NonDestroyed))
  ;[1 1 1] Dammage with linetrace and destruction
  (bind _returnvalue (Niagara|SpawnSystematLocation "/Game/NIAGARA_System/Particles/NS_DestructibleGlass.NS_DestructibleGlass" (Transformation|GetWorldLocation _glasswall_nondestroyed) (Transformation|GetWorldRotation _glasswall_nondestroyed) (Transformation|GetWorldScale _glasswall_nondestroyed)))
  (Components|DestroyComponent (Variables|Default|GetGlassWall_NonDestroyed))
  (EventDispatchers|BindEventtoOnSystemFinished _returnvalue (delegate Custom|Destroy_Glass))
  (Audio|PlaySoundatLocation "/Game/Sounds/glass-break-bounce_E_major.glass-break-bounce_E_major" (Transformation|GetActorLocation) "0, 0, 0" 1.0 1.0 0.0 0 0 0 0))

(fn ConstructionScript)