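; BP_Door is an interactable door that the player opens and closes, with a HUD prompt matching its current state.
; Interact toggles a Status enum between Closed and Open and plays or reverses the Door_Mechanics timeline.
; The timeline's DoorZRotation track drives the static mesh's relative yaw, so closing reuses the opening animation backwards.
; ShowInfo sets the HUD info text to an open or close hint based on Status.
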(event EventBeginPlay)

(event Collision|EventActorBeginOverlap
  (params (OtherActor :type Actor%20Object%20Reference)))

(event EventTick
  (params (DeltaSeconds :type Float%20%28single-precision%29)))

(event EventInteract
  ;[1 0.3385 0.3385] Interact Function
  (switch Utilities|FlowControl|Switch|SwitchonEn_DoorStatus (Variables|Default|GetStatus)
    (:NewEnumerator0
      (Variables|Default|SetStatus "NewEnumerator1")
      (bind _door_z_rotation (Timeline|Door_Mechanics Play)
        (:Update
          (Transformation|SetRelativeRotation (Variables|Default|GetStaticMesh) (Math|Rotator|MakeRotator 0.0 0.0 _door_z_rotation) false false))))
    (:NewEnumerator1
      (Variables|Default|SetStatus "NewEnumerator0")
      (Timeline|Door_Mechanics Reverse))))

(event EventShowInfo
  (params (HUD :type WBP%20HUD%20Object%20Reference))
  ;[0.06297 0.2832 1] Display text to the player
  (switch Utilities|FlowControl|Switch|SwitchonEn_DoorStatus (Variables|Default|GetStatus)
    (:NewEnumerator0
      (Default|SetInfoText HUD "Press [E] to open the door"))
    (:NewEnumerator1
      (Default|SetInfoText HUD "Press [E] to close the door"))))

(fn ConstructionScript)