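; BP_CoffreFort is an interactable safe that opens only when all three of its code checks are valid.
; The Chest_Open event tests IsCodeValid on Code1, Code2 and Code3, then plays the ChestOpen timeline.
; The timeline lerps the Chest component's yaw to a quarter turn and fires a sliding-door sound at the actor's location on every update tick, rather than once.
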(event Custom|Chest_Open
  (if (Math|Boolean|ANDBoolean (Variables|/Game/Interactable_Objects/BP_CadenasBase.BP_CadenasBase_C|GetIsCodeValid (Variables|Default|GetCode1)) (Variables|/Game/Interactable_Objects/BP_CadenasBase.BP_CadenasBase_C|GetIsCodeValid (Variables|Default|GetCode2)) (Variables|/Game/Interactable_Objects/BP_CadenasBase.BP_CadenasBase_C|GetIsCodeValid (Variables|Default|GetCode3)))
    (bind _chestopen (Timeline|ChestOpen Play)
      (:Update
        (Transformation|SetRelativeRotation (Variables|Default|GetChest) (Math|Rotator|MakeRotator 0.0 0.0 (Math|Float|Lerp 0.0 -9e+01 _chestopen)) false false)
        (Audio|PlaySoundatLocation "/Game/Sounds/mixkit-wooden-long-sliding-door-191.mixkit-wooden-long-sliding-door-191" (Transformation|GetActorLocation) "0, 0, 0" 1.0 1.0 0.0 0 0 0 0)))))

(fn ConstructionScript)