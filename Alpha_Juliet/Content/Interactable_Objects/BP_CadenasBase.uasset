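; BP_CadenasBase is an interactable padlock with a four-position rotating dial that opens a linked chest on the correct code.
; Overlapping its collision box registers it as the third-person character's target padlock and enables interaction; leaving disables interaction but keeps that reference.
; Rotate_Upward rolls the cube a quarter turn, cycles the position, updates code validity and calls ChestOpen on the target chest when it matches.
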(event OnComponentBeginOverlap(Box_Collision)
  (params (OverlappedComponent :type Primitive%20Component%20Object%20Reference) (OtherActor :type Actor%20Object%20Reference) (OtherComp :type Primitive%20Component%20Object%20Reference) (OtherBodyIndex :type Integer) (bFromSweep :type Boolean) (SweepResult :type Hit%20Result%20Structure%20%28by%20ref%29))
  (bind _asbp_third_person_character (Utilities|Casting|CastToBP_ThirdPersonCharacter OtherActor))
  (Variables|/Game/ThirdPerson/Blueprints/BP_ThirdPersonCharacter.BP_ThirdPersonCharacter_C|SetTarget_Cadenas _asbp_third_person_character self)
  (Variables|Default|SetCan_Interact? true))

(event OnComponentEndOverlap(Box_Collision)
  (params (OverlappedComponent :type Primitive%20Component%20Object%20Reference) (OtherActor :type Actor%20Object%20Reference) (OtherComp :type Primitive%20Component%20Object%20Reference) (OtherBodyIndex :type Integer))
  ;[1 1 1] End of interaction for cadenas
  (Utilities|Casting|CastToBP_ThirdPersonCharacter OtherActor)
  (Variables|Default|SetCan_Interact? false))

(event Custom|Rotate_Upward
  (bind _cube (Variables|Default|GetCube))
  (bind _relativerotation (Variables|/Script/Engine.SceneComponent|GetRelativeRotation _cube))
  (if (Variables|Default|GetCan_Interact?)
    (Transformation|SetRelativeRotation _cube (Math|Rotator|MakeRotator (+ 9e+01 (.roll _relativerotation)) (.pitch _relativerotation) (.yaw _relativerotation)) false false)
    (if (== (Variables|Default|GetCurrentPosition) 4)
      (Variables|Default|SetCurrentPosition 1)
      (else
        (Variables|Default|SetCurrentPosition (+ (Variables|Default|GetCurrentPosition) 1))))
    (if (== (Variables|Default|GetValid_Code) (Variables|Default|GetCurrentPosition))
      (Variables|Default|SetIsCodeValid true)
      (bind _targetchest (Variables|Default|GetTargetChest)
        (:then
          (Default|ChestOpen _targetchest))
        (:else))
      (else
        (Variables|Default|SetIsCodeValid false)))))

(fn ConstructionScript)